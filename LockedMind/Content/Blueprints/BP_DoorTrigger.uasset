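; BP_DoorTrigger is a trigger volume that opens or closes a referenced door when the first-person character enters it.
; The Box overlap checks CanTrigger, then passes through a DoOnce so the door is driven only once.
; WillOpen selects the action on MyDoor: opening sets IsOpen, while closing clears IsOpen and also makes the door non-interactable.
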(event OnComponentBeginOverlap(Box)
  (params (OverlappedComponent :type Primitive%20Component%20Object%20Reference) (OtherActor :type Actor%20Object%20Reference) (OtherComp :type Primitive%20Component%20Object%20Reference) (OtherBodyIndex :type Integer) (bFromSweep :type Boolean) (SweepResult :type Hit%20Result%20Structure%20%28by%20ref%29))
  (bind _mydoor (Variables|Default|GetMyDoor))
  (Utilities|Casting|CastToFirstPersonCharacter OtherActor)
  (if (Variables|Default|GetCanTrigger)
    (Utilities|FlowControl|DoOnce false
      (:Completed
        (if (Variables|Default|GetWillOpen)
          (Default|OpenDoor (Variables|Default|GetMyDoor))
          (Variables|/Game/Blueprints/BP_Door.BP_Door_C|SetIsOpen (Variables|Default|GetMyDoor) true)
          (else
            (Default|CloseDoor (Variables|Default|GetMyDoor))
            (Variables|/Game/Blueprints/BP_Door.BP_Door_C|SetIsOpen _mydoor false)
            (Variables|/Game/Blueprints/BP_Door.BP_Door_C|SetIsInteractable _mydoor false)))))))

(event EventBeginPlay)

(event Collision|EventActorBeginOverlap
  (params (OtherActor :type Actor%20Object%20Reference)))

(event EventTick
  (params (DeltaSeconds :type Float%20%28single-precision%29)))

(fn ConstructionScript)