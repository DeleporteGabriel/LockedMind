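; BP_StressZone is a box-shaped area that drains the player's sanity while a FirstPersonCharacter stands inside it.
; Tick runs through a short Delay to throttle the overlap poll, then calls LoseSanity on player 0's BP_MyPlayerController.
; The construction script scales the box from the Dimentions variable, so the zone's size is set by that variable.
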(event EventTick
  (params (DeltaSeconds :type Float%20%28single-precision%29))
  (Utilities|FlowControl|Delay 0.05)
  (Utilities|IsValid (Utilities|Array|Get(acopy) (Collision|GetOverlappingActors (Variables|Default|GetBox) "/Game/FirstPersonBP/Blueprints/FirstPersonCharacter.FirstPersonCharacter_C" :!class /Script/Engine.PrimitiveComponent))
    (:Is%20Valid
      (bind _asbp_my_player_controller (Utilities|Casting|CastToBP_MyPlayerController (Game|GetPlayerController 0)))
      (Default|LoseSanity _asbp_my_player_controller 1))))

(fn ConstructionScript
  (Transformation|SetRelativeScale3D (Variables|Default|GetBox) (Variables|Default|GetDimentions)))