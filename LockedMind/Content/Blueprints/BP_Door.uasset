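; BP_Door is an interactable door that toggles between two rotations when WhenInteracted is called and IsActivate is true.
; A timeline plays forward to open and reverses to close, lerping the root's world rotation from RotationOpen to RotationClose, so those names read inverted relative to IsOpen.
; The construction script poses the door from IsOpen, and BeginPlay moves the timeline to 1.0 for doors that start open.
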(event Custom|OpenDoor
  (bind _lerp (Timeline|OpenDoorTimeline Play)
    (:Update
      (Transformation|SetWorldRotation (Variables|Default|GetDefaultSceneRoot) (Math|Rotator|Lerp(Rotator) (Variables|Default|GetRotationOpen) (Variables|Default|GetRotationClose) _lerp) false false))))

(event Custom|CloseDoor
  (bind _lerp (Timeline|OpenDoorTimeline Reverse)
    (:Update
      (Transformation|SetWorldRotation (Variables|Default|GetDefaultSceneRoot) (Math|Rotator|Lerp(Rotator) (Variables|Default|GetRotationOpen) (Variables|Default|GetRotationClose) _lerp) false false))))

(event EventBeginPlay
  (if (Variables|Default|GetIsOpen)
    (Components|Timeline|SetNewTime (Variables|Default|GetOpenDoorTimeline) 1.0)))

(event Collision|EventActorBeginOverlap
  (params (OtherActor :type Actor%20Object%20Reference)))

(event EventTick
  (params (DeltaSeconds :type Float%20%28single-precision%29)))

(fn ConstructionScript
  (|CallParentFunction)
  (if (Variables|Default|GetIsOpen)
    (Transformation|SetWorldRotation (Variables|Default|GetDefaultSceneRoot) (Variables|Default|GetRotationClose) false false)
    (else
      (Transformation|SetWorldRotation (Variables|Default|GetDefaultSceneRoot) (Variables|Default|GetRotationOpen) false false))))

(fn WhenInteracted
  (if (Variables|Default|GetIsActivate)
    (if (Variables|Default|GetIsOpen)
      (CallFunction|CloseDoor)
      (Variables|Default|SetIsOpen false)
      (else
        (CallFunction|OpenDoor)
        (Variables|Default|SetIsOpen true)))))