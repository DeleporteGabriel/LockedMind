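; BP_DialogueMaker is a trigger actor that plays a timed sequence of dialogue lines when the first-person character enters its box.
; An overlap, gated by an activation flag and a DoOnce, fires TriggerDialogue, which adds the player controller's dialogue UI to the viewport.
; A looped Delay steps through parallel line and delay arrays, sending each line to the controller, then removes the UI.
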(event OnComponentBeginOverlap(Box)
  (params (OverlappedComponent :type Primitive%20Component%20Object%20Reference) (OtherActor :type Actor%20Object%20Reference) (OtherComp :type Primitive%20Component%20Object%20Reference) (OtherBodyIndex :type Integer) (bFromSweep :type Boolean) (SweepResult :type Hit%20Result%20Structure%20%28by%20ref%29))
  (Utilities|Casting|CastToBP_FirstPersonCharacter OtherActor)
  (if (Variables|Default|GetIsActivate)
    (Utilities|FlowControl|DoOnce false
      (:Completed
        (CallFunction|TriggerDialogue)))))

(event Custom|TriggerDialogue
  (bind _asbp_my_player_controller (Utilities|Casting|CastToBP_MyPlayerController (Game|GetPlayerController 0)))
  (UserInterface|Viewport|AddtoViewport (Variables|/Game/Blueprints/BP_MyPlayerController.BP_MyPlayerController_C|GetDialogueUI _asbp_my_player_controller) 0)
  (if (< (Variables|Default|GetDialogueStep) (Utilities|Array|Length (Variables|Default|GetDialogueList))) :!label _label
    (Default|DisplayDialogue _asbp_my_player_controller (Utilities|Array|Get(acopy) (Variables|Default|GetDialogueList) (Variables|Default|GetDialogueStep)))
    (Utilities|FlowControl|Delay (Utilities|Array|Get(acopy) (Variables|Default|GetDialogueDelay) (Variables|Default|GetDialogueStep)))
    (Variables|Default|SetDialogueStep (+ (Variables|Default|GetDialogueStep) 1))
    (goto _label)
    (else
      (Widget|RemovefromParent (Variables|/Game/Blueprints/BP_MyPlayerController.BP_MyPlayerController_C|GetDialogueUI _asbp_my_player_controller)))))

(fn ConstructionScript)