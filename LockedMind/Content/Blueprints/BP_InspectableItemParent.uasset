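; BP_InspectableItemParent is a base Blueprint for items the player inspects and rotates with the mouse.
; While left or right mouse button is held, mouse X adds inverted roll and mouse Y inverted pitch to the root's relative rotation.
; CombineRotators composes each delta onto the current rotation.
; Pressing G disables the item's input and calls StopInspecting on the FirstPersonCharacter to end inspection.
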(event Input|MouseEvents|MouseX
  (params (AxisValue :type Float%20%28single-precision%29))
  (bind _returnvalue (Game|GetPlayerController 0))
  ;[1 1 1] Rotation
  (if (or (Game|Player|IsInputKeyDown _returnvalue "LeftMouseButton") (Game|Player|IsInputKeyDown _returnvalue "RightMouseButton"))
    (Transformation|SetRelativeRotation (Variables|Default|GetDefaultSceneRoot) (Math|Rotator|CombineRotators (Variables|/Script/Engine.SceneComponent|GetRelativeRotation (Variables|Default|GetDefaultSceneRoot)) (Math|Rotator|MakeRotator (* AxisValue -1.0) 0.0 0.0)) false false)))

(event Input|MouseEvents|MouseY
  (params (AxisValue :type Float%20%28single-precision%29))
  (bind _returnvalue (Game|GetPlayerController 0))
  ;[1 1 1] Rotation
  (if (or (Game|Player|IsInputKeyDown _returnvalue "LeftMouseButton") (Game|Player|IsInputKeyDown _returnvalue "RightMouseButton"))
    (Transformation|SetRelativeRotation (Variables|Default|GetDefaultSceneRoot) (Math|Rotator|CombineRotators (Variables|/Script/Engine.SceneComponent|GetRelativeRotation (Variables|Default|GetDefaultSceneRoot)) (Math|Rotator|MakeRotator 0.0 (* AxisValue -1.0) 0.0)) false false)))

(event Input|KeyboardEvents|G
  (params (Key :type Key%20Structure :default "None"))
  ;[1 1 1] Inspection
  (:Pressed
    (Input|DisableInput (Game|GetPlayerController 0))
    (bind _asfirst_person_character (Utilities|Casting|CastToFirstPersonCharacter (Game|Player|GetPlayerPawn 0)))
    (Default|StopInspecting _asfirst_person_character)))

(fn ConstructionScript)