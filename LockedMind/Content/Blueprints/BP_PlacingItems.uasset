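; BP_PlacingItems is an interactable with four emplacements where the player places items from their inventory.
; Interaction alternates between opening the inventory and closing it, with the latter moving the first held item to the next emplacement.
; The placed item becomes visible and non-pickable, plays a Niagara effect, activates its linked triggers, dialogues, doors and sublevels, then leaves the inventory.
; Once the placement counter reaches four, the player controller's MoveInOrderActivate runs.
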(event EventBeginPlay
  (Utilities|Array|Add (Variables|Default|GetEmplacements) (Variables|Default|GetEmplacement1))
  (Utilities|Array|Add (Variables|Default|GetEmplacements) (Variables|Default|GetEmplacement2))
  (Utilities|Array|Add (Variables|Default|GetEmplacements) (Variables|Default|GetEmplacement3))
  (Utilities|Array|Add (Variables|Default|GetEmplacements) (Variables|Default|GetEmplacement4)))

(fn ConstructionScript
  (|CallParentFunction))

(fn WhenInteracted
  (bind _asbp_my_player_controller (Utilities|Casting|CastToBP_MyPlayerController (Game|GetPlayerController 0)))
  (if (Variables|Default|GetIsUsed)
    (bind _asbp_my_player_controller_2 (Utilities|Casting|CastToBP_MyPlayerController (Game|GetPlayerController 0)))
    (if (> (Utilities|Array|Length (Variables|/Game/Blueprints/BP_MyPlayerController.BP_MyPlayerController_C|GetInventory _asbp_my_player_controller_2)) 0)
      (Transformation|SetWorldLocationAndRotation (Variables|/Game/Blueprints/BP_InspectableItemParent.BP_InspectableItemParent_C|GetDefaultSceneRoot (Utilities|Array|Get(acopy) (Variables|/Game/Blueprints/BP_MyPlayerController.BP_MyPlayerController_C|GetInventory _asbp_my_player_controller_2))) (Transformation|GetWorldLocation (Utilities|Array|Get(acopy) (Variables|Default|GetEmplacements) (Variables|Default|GetPlacedObject))) "0, 0, 0" false false)
      (Niagara|SpawnSystematLocation "/Game/Assets/FX/NS_KeyObjectPlaced.NS_KeyObjectPlaced" (Transformation|GetWorldLocation (Utilities|Array|Get(acopy) (Variables|Default|GetEmplacements) (Variables|Default|GetPlacedObject))))
      (Rendering|SetVisibility (Variables|/Game/Blueprints/BP_InspectableItemParent.BP_InspectableItemParent_C|GetItem (Utilities|Array|Get(acopy) (Variables|/Game/Blueprints/BP_MyPlayerController.BP_MyPlayerController_C|GetInventory _asbp_my_player_controller_2))) true false)
      (Variables|/Game/Blueprints/BP_InspectableItemParent.BP_InspectableItemParent_C|SetCanBePicked (Utilities|Array|Get(acopy) (Variables|/Game/Blueprints/BP_MyPlayerController.BP_MyPlayerController_C|GetInventory _asbp_my_player_controller_2)) false)
      (|SetActivate (Utilities|Array|Get(acopy) (Variables|/Game/Blueprints/BP_MyPlayerController.BP_MyPlayerController_C|GetInventory _asbp_my_player_controller_2))
        (:Completed
          (Utilities|Array|RemoveIndex (Variables|/Game/Blueprints/BP_MyPlayerController.BP_MyPlayerController_C|GetInventory _asbp_my_player_controller_2)))))
    (Variables|Default|SetIsUsed false)
    (Default|ClosetheInventory _asbp_my_player_controller)
    (Variables|Default|SetPlacedObject (+ (Variables|Default|GetPlacedObject) 1))
    (if (>= (Variables|Default|GetPlacedObject) 4)
      (Default|MoveinOrderActivate _asbp_my_player_controller))
    (else
      (Variables|Default|SetIsUsed true)
      (Default|OpentheInventory _asbp_my_player_controller))))