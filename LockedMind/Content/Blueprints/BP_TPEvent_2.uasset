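; BP_TPEvent_2 is an interactable that triggers the game's ending once the player has placed at least four objects.
; On interaction it sets a new respawn point, teleports the player behind a black screen and swaps the streamed level from MansionV3 to TutorialLevel.
; It then plays the ending dialogue and Lynch audio, and after a timed wait fades the black screen through a timeline and quits the game.
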(event Custom|DelayThenRemove
  (params (Target :type Widget%20Object%20Reference))
  (Game|LoadStreamLevel(byName) "TutorialLevel" true)
  (Utilities|FlowControl|Delay 1.0)
  (Widget|RemovefromParent Target)
  (Game|UnloadStreamLevel(byName) "MansionV3" false)
  (Default|TriggerDialogue (Variables|Default|GetEndingDialogue))
  (Audio|PlaySoundatLocation "/Game/Audio/Dialogues/A_Lynch_ending.A_Lynch_ending" (Transformation|GetWorldLocation (Variables|/Script/Engine.Actor|GetRootComponent (Variables|Default|GetLynchPosition))) "0, 0, 0" 1.0 1.0 0.0 "/Game/Audio/ATT_Base.ATT_Base" 0 0)
  (Utilities|FlowControl|Delay 13.5)
  (UserInterface|Viewport|AddtoViewport (Variables|Default|GetBlackScreen) 0)
  (bind _newtrack_0 (Timeline|Fondu Play)
    (:Update
      (Default|UpdateOpacity (Variables|Default|GetBlackScreen) _newtrack_0))
    (:Finished
      (Game|QuitGame 0 "Quit" false))))

(event EventBeginPlay)

(event Collision|EventActorBeginOverlap
  (params (OtherActor :type Actor%20Object%20Reference)))

(event EventTick
  (params (DeltaSeconds :type Float%20%28single-precision%29)))

(fn ConstructionScript
  (|CallParentFunction))

(fn WhenInteracted
  (bind _asbp_my_player_controller (Utilities|Casting|CastToBP_MyPlayerController (Game|GetPlayerController 0)))
  (if (>= (Variables|/Game/Blueprints/BP_MyPlayerController.BP_MyPlayerController_C|GetPlacedObject _asbp_my_player_controller) 4)
    (Variables|/Game/Blueprints/BP_FirstPersonCharacter.BP_FirstPersonCharacter_C|SetRespawnPoint (Variables|/Game/Blueprints/BP_MyPlayerController.BP_MyPlayerController_C|GetMyPlayer _asbp_my_player_controller) (Variables|Default|GetMyRespawn))
    (bind _returnvalue (UserInterface|CreateWidget "/Game/Blueprints/Widgets/WBP_BlackScreen.WBP_BlackScreen_C"))
    (Variables|Default|SetBlackScreen _returnvalue)
    (UserInterface|Viewport|AddtoViewport _returnvalue 0)
    (Transformation|SetWorldLocation (Variables|/Script/Engine.Character|GetCapsuleComponent (Variables|/Game/Blueprints/BP_MyPlayerController.BP_MyPlayerController_C|GetMyPlayer _asbp_my_player_controller)) (Transformation|GetWorldLocation (Variables|/Script/Engine.Actor|GetRootComponent (Variables|Default|GetTPlocation))) false true)
    (CallFunction|DelayThenRemove _returnvalue)))