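; BP_TutoMecanique scripts a mechanics tutorial built around a key item and dialogue triggers.
; On BeginPlay it hides the key, triggers the first dialogue and freezes player movement briefly.
; When the player controller's GagneMJStress event fires, it reveals the key and triggers the second dialogue.
; That event is reassigned every Tick rather than once, and a delayed CanBreath unlock is left unconnected.
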(event Custom|GagneMJStress_Event_0
  (Rendering|SetActorHiddenInGame (Variables|Default|GetMyKeyItem) false)
  (Default|TriggerDialogue (Utilities|Array|Get(acopy) (Variables|Default|GetMyStartingDialogue) 1)))

(event EventTick
  (params (DeltaSeconds :type Float%20%28single-precision%29))
  (bind _asbp_my_player_controller (Utilities|Casting|CastToBP_MyPlayerController (Game|GetPlayerController 0)))
  (EventDispatchers|AssignGagneMJStress _asbp_my_player_controller (delegate Custom|GagneMJStress_Event_0)))

(event EventBeginPlay
  (Rendering|SetActorHiddenInGame (Variables|Default|GetMyKeyItem) true)
  (Default|TriggerDialogue (Utilities|Array|Get(acopy) (Variables|Default|GetMyStartingDialogue)))
  (bind _asbp_my_player_controller (Utilities|Casting|CastToBP_MyPlayerController (Game|GetPlayerController 0)))
  (bind _output_get (Variables|Default|SetMyPlayer (Variables|/Game/Blueprints/BP_MyPlayerController.BP_MyPlayerController_C|GetMyPlayer _asbp_my_player_controller)))
  (Variables|/Game/Blueprints/BP_FirstPersonCharacter.BP_FirstPersonCharacter_C|SetCanMove _output_get false)
  (Utilities|FlowControl|Delay 3.0)
  (Variables|/Game/Blueprints/BP_FirstPersonCharacter.BP_FirstPersonCharacter_C|SetCanMove _output_get true))

(fn ConstructionScript)