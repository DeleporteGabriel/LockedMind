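; BP_EventVisual is a triggerable visual event: a configurable mesh, hidden at play start, that appears and moves when DoWhenTrigger runs.
; A timeline, its play rate set by MovementSpeed, lerps the mesh's relative location and world rotation from start to end values.
; After the movement finishes, it waits Duration seconds and hides again.
; The construction script applies the mesh and previews the start or end pose through ShowEndingPos.
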(event Custom|Reappearance
  (bind _lerp (Timeline|TimelineMouvement PlayFromStart)
    (:Update
      (Transformation|SetRelativeLocation (Variables|Default|GetCube) (Math|Vector|Lerp(Vector) (Variables|Default|GetEventLocationStart) (Variables|Default|GetEventLocationEnd) _lerp) false false)
      (Transformation|SetWorldRotation (Variables|Default|GetCube) (Math|Rotator|Lerp(Rotator) (Variables|Default|GetEventRotationStart) (Variables|Default|GetEventRotationEnd) _lerp) false false))
    (:Finished
      (Utilities|FlowControl|Delay (Variables|Default|GetDuration))
      (Rendering|SetVisibility (Variables|Default|GetCube) false false))))

(event EventBeginPlay
  (Rendering|SetVisibility (Variables|Default|GetCube) false false)
  (Components|Timeline|SetPlayRate (Variables|Default|GetTimelineMouvement) (Variables|Default|GetMovementSpeed)))

(fn ConstructionScript
  (|CallParentFunction)
  (Components|StaticMesh|SetStaticMesh (Variables|Default|GetCube) (Variables|Default|GetModele))
  (if (not (Variables|Default|GetShowEndingPos))
    (Transformation|SetRelativeLocation (Variables|Default|GetCube) (Variables|Default|GetEventLocationStart) false false)
    (Transformation|SetWorldRotation (Variables|Default|GetCube) (Variables|Default|GetEventRotationStart) false false)
    (else
      (Transformation|SetRelativeLocation (Variables|Default|GetCube) (Variables|Default|GetEventLocationEnd) false false)
      (Transformation|SetWorldRotation (Variables|Default|GetCube) (Variables|Default|GetEventRotationEnd) false false))))

(fn DowhenTrigger
  (Rendering|SetVisibility (Variables|Default|GetCube) true false)
  (CallFunction|Reappearance))