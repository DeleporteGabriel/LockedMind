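; BP_TPEvent is an interaction-triggered event that teleports the player and swaps streamed mansion levels behind a black screen.
; WhenInteracted shows WBP_BlackScreen, then moves the player's capsule to the arrow on TPlocation.
; DelayThenRemove starts non-blocking loads of MansionV1 and IntermediateV2_3, waits briefly, removes the screen and unloads MansionV2 and IntermediateV1_2.
; Level names are hardcoded, and the fixed delay does not wait for streaming to finish.
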(event Custom|DelayThenRemove
  (params (Target :type Widget%20Object%20Reference))
  (Game|LoadStreamLevel(byName) "MansionV1" true)
  (Game|LoadStreamLevel(byName) "IntermediateV2_3" true)
  (Utilities|FlowControl|Delay 1.0)
  (Widget|RemovefromParent Target)
  (Game|UnloadStreamLevel(byName) "MansionV2" false)
  (Game|UnloadStreamLevel(byName) "IntermediateV1_2" false))

(event EventBeginPlay)

(event Collision|EventActorBeginOverlap
  (params (OtherActor :type Actor%20Object%20Reference)))

(event EventTick
  (params (DeltaSeconds :type Float%20%28single-precision%29)))

(fn ConstructionScript
  (|CallParentFunction))

(fn WhenInteracted
  (bind _asbp_my_player_controller (Utilities|Casting|CastToBP_MyPlayerController (Game|GetPlayerController 0)))
  (bind _returnvalue (UserInterface|CreateWidget "/Game/Blueprints/Widgets/WBP_BlackScreen.WBP_BlackScreen_C"))
  (UserInterface|Viewport|AddtoViewport _returnvalue 0)
  (Transformation|SetWorldLocation (Variables|/Script/Engine.Character|GetCapsuleComponent (Variables|/Game/Blueprints/BP_MyPlayerController.BP_MyPlayerController_C|GetMyPlayer _asbp_my_player_controller)) (Transformation|GetWorldLocation (Variables|/Script/Engine.TargetPoint|GetArrowComponent (Variables|Default|GetTPlocation))) false true)
  (CallFunction|DelayThenRemove _returnvalue))