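; BP_EventTriggerParent is a base trigger volume that fires a one-time event and calls LoseStress on the player controller.
; When the first-person character overlaps the box while CanTrigger is set, a DoOnce gate passes StressPoints to BP_MyPlayerController.
; It then calls DoWhenTrigger, an empty hook apparently meant for child Blueprints to override.
; The construction script scales the box from TriggerSize.
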(event OnComponentBeginOverlap(triggerbox)
  (params (OverlappedComponent :type Primitive%20Component%20Object%20Reference) (OtherActor :type Actor%20Object%20Reference) (OtherComp :type Primitive%20Component%20Object%20Reference) (OtherBodyIndex :type Integer) (bFromSweep :type Boolean) (SweepResult :type Hit%20Result%20Structure%20%28by%20ref%29))
  (Utilities|Casting|CastToBP_FirstPersonCharacter OtherActor)
  (if (Variables|Default|GetCanTrigger)
    (Utilities|FlowControl|DoOnce false
      (:Completed
        (bind _asbp_my_player_controller (Utilities|Casting|CastToBP_MyPlayerController (Game|GetPlayerController 0)))
        (Default|LoseStress _asbp_my_player_controller (Variables|Default|GetStressPoints))
        (CallFunction|DowhenTrigger)))))

(fn ConstructionScript
  (Transformation|SetWorldScale3D (Variables|Default|Gettriggerbox) (Variables|Default|GetTriggerSize)))

(fn DowhenTrigger)