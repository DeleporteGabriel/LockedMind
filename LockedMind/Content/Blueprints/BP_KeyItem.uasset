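; BP_KeyItem is a key item the player collects by pressing E, adding it to the controller's inventory.
; Collecting it records it as the last held item, ends the player's inspection, restores movement, and activates linked objects in ActivateWhenGrab.
; Items with a puzzle launch a jigsaw through the controller, guarded by a DoOnce that JigsawL resets, optionally followed by timed hint dialogue about nightmares and memories.
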(event Custom|JigsawL
  (Utilities|FlowControl|DoOnce false) ; enters at Reset
)

(event Input|KeyboardEvents|E
  (params (Key :type Key%20Structure :default "None"))
  (bind _returnvalue (Game|GetPlayerController 0))
  (:Pressed
    (Input|DisableInput _returnvalue)
    (bind _asbp_my_player_controller (Utilities|Casting|CastToBP_MyPlayerController _returnvalue))
    (Variables|/Game/Blueprints/BP_MyPlayerController.BP_MyPlayerController_C|SetLastHoldedKeyItem _asbp_my_player_controller self)
    (Default|AddIteminInventory _asbp_my_player_controller self)
    (Variables|/Game/Blueprints/BP_FirstPersonCharacter.BP_FirstPersonCharacter_C|SetHoldedItem (Variables|/Game/Blueprints/BP_MyPlayerController.BP_MyPlayerController_C|GetMyPlayer _asbp_my_player_controller) 0)
    (Variables|/Game/Blueprints/BP_FirstPersonCharacter.BP_FirstPersonCharacter_C|SetInspecting? (Variables|/Game/Blueprints/BP_MyPlayerController.BP_MyPlayerController_C|GetMyPlayer _asbp_my_player_controller) false)
    (Variables|/Game/Blueprints/BP_FirstPersonCharacter.BP_FirstPersonCharacter_C|SetCanMove (Variables|/Game/Blueprints/BP_MyPlayerController.BP_MyPlayerController_C|GetMyPlayer _asbp_my_player_controller) true)
    (Default|StopCollect (Variables|/Game/Blueprints/BP_MyPlayerController.BP_MyPlayerController_C|GetMyPlayer _asbp_my_player_controller))
    (for _array_element (Variables|Default|GetActivateWhenGrab)
      (Variables|/Game/Blueprints/BP_CanBeActivateParent.BP_CanBeActivateParent_C|SetIsActivate _array_element true))
    (if (Variables|Default|GetHavePuzzle)
      (Utilities|FlowControl|DoOnce false
        (:Completed
          (Default|JigsawActivate _asbp_my_player_controller (Variables|Default|GetPuzzleTextures))
          (if (Variables|Default|GetDialogueLynch)
            (UserInterface|Viewport|AddtoViewport (Variables|/Game/Blueprints/BP_MyPlayerController.BP_MyPlayerController_C|GetDialogueUI _asbp_my_player_controller) 0)
            (Default|DisplayDialogue _asbp_my_player_controller "What this object mean to you ? Try to connect your nightmare with your personal memories. ")
            (Utilities|FlowControl|Delay 4.0)
            (Default|DisplayDialogue _asbp_my_player_controller "Nightmares often refer to elements of our lives.")
            (Utilities|FlowControl|Delay 2.0)
            (Widget|RemovefromParent (Variables|/Game/Blueprints/BP_MyPlayerController.BP_MyPlayerController_C|GetDialogueUI _asbp_my_player_controller))))))))

(fn ConstructionScript
  (|CallParentFunction))