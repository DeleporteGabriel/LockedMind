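; Player controller for a first-person game, running the stress/sanity system, inventory, dialogue and puzzle widgets.
; CurrentStress works as sanity, driving the stress bar, BPM text and walk speed; at zero the player drops the first inventory item and respawns.
; H toggles a timing minigame where J presses inside a randomized timeline window restore sanity and misses cost it.
; Puzzle screens lock movement, and an open jigsaw steadily drains sanity.
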(event Custom|CallSanityRecovery
  ;[1 1 1] RecoverSanity
  (if (Variables|Stress|GetStressRecovery)
    (Variables|/Script/Engine.CharacterMovementComponent|SetMaxWalkSpeed (Variables|/Script/Engine.Character|GetCharacterMovement (Variables|Default|GetMyPlayer)) (* (Variables|Default|GetBaseSpeed) (Utilities|GetSanityPercent)))
    (Widget|RemovefromParent (Variables|UI|GetRecoverUI))
    (Default|FlipArm (Variables|Default|GetMyPlayer))
    (Variables|Stress|SetStressRecovery false)
    (bind _cursortrack (Timeline|RecoveryTimeline Stop)
      (:Update
        (Default|UpdateRecoveryBar (Variables|UI|GetRecoverUI) _cursortrack)
        (Variables|RecoverGame|SetRecoveryTrack _cursortrack)))
    (else
      (UserInterface|Viewport|AddtoViewport (Variables|UI|GetRecoverUI) 0)
      (Default|FlipArm (Variables|Default|GetMyPlayer))
      (CallFunction|UpdateStressMarge)
      (Variables|Stress|SetStressRecovery true)
      (Timeline|RecoveryTimeline PlayFromStart))))

(event Custom|AddItemInInventory
  (params (NewItem :type BP%20Key%20Item%20Object%20Reference%20%28by%20ref%29))
  (Utilities|Array|Add (Variables|Default|GetInventory) NewItem)
  (Rendering|SetVisibility (Variables|/Game/Blueprints/BP_InspectableItemParent.BP_InspectableItemParent_C|GetItem NewItem) false false)
  (Transformation|SetWorldLocation (Variables|/Game/Blueprints/BP_InspectableItemParent.BP_InspectableItemParent_C|GetDefaultSceneRoot NewItem) "0.000000, 0,-1000.000000" false true)
  (Development|PrintString "Item added"))

(event Custom|SetCursorSpeed
  (params (NewRate :type Float%20%28single-precision%29))
  (Components|Timeline|SetPlayRate (Variables|Default|GetRecoveryTimeline) NewRate))

(event Custom|JigsawDeactivate
  (Widget|RemovefromParent (Variables|UI|GetJigsawUI))
  (Variables|Default|SetbShowMouseCursor false)
  (Variables|/Game/Blueprints/BP_FirstPersonCharacter.BP_FirstPersonCharacter_C|SetCanMove (Variables|Default|GetMyPlayer) true)
  (Variables|UI|SetJigsawUI 0))

(event Custom|OpenTheInventory
  (UserInterface|Viewport|AddtoViewport (Variables|UI|GetInventoryWBP) 0)
  (Variables|/Game/Blueprints/BP_FirstPersonCharacter.BP_FirstPersonCharacter_C|SetCanMove (Variables|Default|GetMyPlayer) false)
  (Default|UpdateObjects (Variables|UI|GetInventoryWBP) self))

(event Custom|CloseTheInventory
  (Variables|/Game/Blueprints/BP_FirstPersonCharacter.BP_FirstPersonCharacter_C|SetCanMove (Variables|Default|GetMyPlayer) true)
  (Widget|RemovefromParent (Variables|UI|GetInventoryWBP)))

(event Custom|DropTheInventory
  (bind _inventory (Variables|Default|GetInventory))
  (bind _myplayer (Variables|Default|GetMyPlayer))
  (bind _output (Utilities|Array|Get(acopy) _inventory))
  (bind _capsulecomponent (Variables|/Script/Engine.Character|GetCapsuleComponent _myplayer))
  (bind _returnvalue (Transformation|GetWorldLocation _capsulecomponent))
  (if (Utilities|IsInventoryEmpty)
    (Transformation|SetWorldLocation (Variables|/Game/Blueprints/BP_InspectableItemParent.BP_InspectableItemParent_C|GetDefaultSceneRoot _output) (Math|Vector|MakeVector (.x _returnvalue) (.y _returnvalue) (- (.z _returnvalue) 96.0)) false true)
    (Rendering|SetVisibility (Variables|/Game/Blueprints/BP_InspectableItemParent.BP_InspectableItemParent_C|GetItem _output) true false)
    (Utilities|Array|Clear (Variables|Default|GetInventory))))

(event Custom|MoveInOrderActivate
  (UserInterface|Viewport|AddtoViewport (Variables|UI|GetPuzzleUI) 0)
  (Variables|Default|SetbShowMouseCursor true)
  (Variables|/Game/Blueprints/BP_FirstPersonCharacter.BP_FirstPersonCharacter_C|SetCanMove (Variables|Default|GetMyPlayer) false))

(event Custom|ResetTimeSinceEvent
  (params (Duration :type Float%20%28single-precision%29))
  (Utilities|FlowControl|RetriggerableDelay Duration)
  (Variables|RecoverGame|SetMJStressRecovered 5)
  (Variables|RecoverGame|SetMJStressLost 1)
  (CallFunction|SetCursorSpeed 2.0))

(event Custom|DisplayDialogue
  (params (DialogueLine :type String))
  (Default|UpdateText (Variables|UI|GetDialogueUI) DialogueLine))

(event Custom|JigsawActivate
  (params (ListTexture :type Array%20of%20Paper%20Sprite%20Object%20References))
  (if (not (Utilities|IsValid (Variables|UI|GetJigsawUI)))
    (bind _returnvalue (UserInterface|CreateWidget "/Game/Blueprints/Widgets/WBP_JigsawGame.WBP_JigsawGame_C"))
    (Variables|UI|SetJigsawUI _returnvalue)
    (UserInterface|Viewport|AddtoViewport (Variables|UI|GetJigsawUI) 0)
    (Default|SetupTextures (Variables|UI|GetJigsawUI) ListTexture)
    (Variables|Default|SetbShowMouseCursor true)
    (Variables|/Game/Blueprints/BP_FirstPersonCharacter.BP_FirstPersonCharacter_C|SetCanMove (Variables|Default|GetMyPlayer) false)))

(event Custom|MoveInOrderDeactivate
  (Widget|RemovefromParent (Variables|UI|GetPuzzleUI))
  (Variables|Default|SetbShowMouseCursor false)
  (Variables|/Game/Blueprints/BP_FirstPersonCharacter.BP_FirstPersonCharacter_C|SetCanMove (Variables|Default|GetMyPlayer) true))

(event EventBeginPlay
  (Utilities|FlowControl|Sequence
    (:then_0
      (Variables|Stress|SetCurrentStress (Variables|Stress|GetStressMax))
      (bind _asbp_first_person_character (Utilities|Casting|CastToBP_FirstPersonCharacter (Game|Player|GetPlayerPawn 0)))
      (Variables|Default|SetMyPlayer _asbp_first_person_character)
      (CallFunction|SetCursorSpeed 2.0))
    (:then_1
      (bind _returnvalue (UserInterface|CreateWidget "/Game/Blueprints/Widgets/WBP_StressBar.WBP_StressBar_C"))
      (bind _output_get (Variables|UI|SetSanityUI _returnvalue))
      (UserInterface|Viewport|AddtoViewport _output_get 0))
    (:then_2
      (bind _returnvalue_2 (UserInterface|CreateWidget "/Game/Blueprints/Widgets/WBP_RecoveryBar.WBP_RecoveryBar_C"))
      (Variables|UI|SetRecoverUI _returnvalue_2)
      (bind _returnvalue_3 (UserInterface|CreateWidget "/Game/Blueprints/Widgets/WBP_Dialogue.WBP_Dialogue_C"))
      (Variables|UI|SetDialogueUI _returnvalue_3))
    (:then_3
      (bind _returnvalue_4 (UserInterface|CreateWidget "/Game/Blueprints/Widgets/WBP_Inventory.WBP_Inventory_C"))
      (Variables|UI|SetInventoryWBP _returnvalue_4))
    (:then_4
      (bind _returnvalue_5 (UserInterface|CreateWidget "/Game/Blueprints/Widgets/WBP_PuzzleGame.WBP_PuzzleGame_C"))
      (Variables|UI|SetPuzzleUI _returnvalue_5))))

(event EventTick
  (params (DeltaSeconds :type Float%20%28single-precision%29))
  (Utilities|FlowControl|Sequence
    (:then_0
      (Utilities|IsValid (Variables|UI|GetJigsawUI)
        (:Is%20Valid
          (Utilities|FlowControl|Delay 1.0)
          (CallFunction|LoseStress 1))))))

(event Input|KeyboardEvents|F
  (params (Key :type Key%20Structure :default "None"))
  (:Pressed
    (CallFunction|LoseStress 10)))

(event Input|KeyboardEvents|H
  (params (Key :type Key%20Structure :default "None"))
  (:Pressed
    (if (Variables|Default|GetCanBreath)
      (CallFunction|CallSanityRecovery))))

(event Input|KeyboardEvents|J
  (params (Key :type Key%20Structure :default "None"))
  ;[1 1 1] RecoverSanity
  (:Pressed
    (if (Variables|Stress|GetStressRecovery)
      (if (and (>= (Variables|RecoverGame|GetRecoveryTrack) (Variables|RecoverGame|GetRecoverRangeMin)) (<= (Variables|RecoverGame|GetRecoveryTrack) (Variables|RecoverGame|GetRecoverRangeMax)))
        (Default|CallGagneMJStress)
        (CallFunction|GainStress (Variables|RecoverGame|GetMJStressRecovered))
        (Variables|/Script/Engine.CharacterMovementComponent|SetMaxWalkSpeed (Variables|/Script/Engine.Character|GetCharacterMovement (Variables|Default|GetMyPlayer)) (* (Variables|Default|GetBaseSpeed) (Utilities|GetSanityPercent)))
        (if (== (Variables|Stress|GetCurrentStress) (Variables|Stress|GetStressMax))
          (Widget|RemovefromParent (Variables|UI|GetRecoverUI))
          (Default|FlipArm (Variables|Default|GetMyPlayer))
          (Variables|Stress|SetStressRecovery false)
          (bind _cursortrack (Timeline|RecoveryTimeline Stop)
            (:Update
              (Default|UpdateRecoveryBar (Variables|UI|GetRecoverUI) _cursortrack)
              (Variables|RecoverGame|SetRecoveryTrack _cursortrack)))
          (else
            (CallFunction|UpdateStressMarge)))
        (else
          (CallFunction|LoseStress (Variables|RecoverGame|GetMJStressLost)))))))

(fn ConstructionScript)

(fn LoseStress
  (params (SanityLost :type Integer))
  (bind _returnvalue (Utilities|GetSanityPercent))
  (bind _returnvalue_2 (Utilities|GetSanityPercent))
  (bind _myplayer (Variables|Default|GetMyPlayer))
  (Variables|Stress|SetCurrentStress (Math|Integer|Clamp(Integer) (- (Variables|Stress|GetCurrentStress) SanityLost) 0 (Variables|Stress|GetStressMax)))
  (Default|UpdateStress (Variables|UI|GetSanityUI) (- 1.0 _returnvalue_2))
  (Rendering|Components|TextRender|SetText (Variables|/Game/Blueprints/BP_FirstPersonCharacter.BP_FirstPersonCharacter_C|GetBPM (Variables|Default|GetMyPlayer)) (Utilities|Text|ToText(Integer) (+ (- (Variables|Stress|GetStressMax) (Variables|Stress|GetCurrentStress)) 80)))
  (if (Variables|Stress|GetStressRecovery)
    _
    (else
      (Variables|/Script/Engine.CharacterMovementComponent|SetMaxWalkSpeed (Variables|/Script/Engine.Character|GetCharacterMovement (Variables|Default|GetMyPlayer)) (* (Variables|Default|GetBaseSpeed) _returnvalue_2))))
  (if (== (Variables|Stress|GetCurrentStress) 0)
    (Development|PrintString "T'es mort loser (L + ratio)")
    ;[1 1 1] Respawned
    (CallFunction|DroptheInventory)
    (Variables|Stress|SetCurrentStress (Variables|Stress|GetStressMax))
    (Transformation|SetActorLocation _myplayer (+ (Transformation|GetWorldLocation (Variables|/Script/Engine.Actor|GetRootComponent (Variables|/Game/Blueprints/BP_FirstPersonCharacter.BP_FirstPersonCharacter_C|GetRespawnPoint _myplayer))) "0, 0,90.000000") false false)
    (Default|UpdateStress (Variables|UI|GetSanityUI) (- 1.0 _returnvalue))
    (Variables|/Script/Engine.CharacterMovementComponent|SetMaxWalkSpeed (Variables|/Script/Engine.Character|GetCharacterMovement (Variables|Default|GetMyPlayer)) (* (Variables|Default|GetBaseSpeed) _returnvalue))
    (Utilities|FlowControl|Sequence
      (:then_0
        (if (Variables|Stress|GetStressRecovery)
          (Widget|RemovefromParent (Variables|UI|GetRecoverUI))
          (Variables|Stress|SetStressRecovery false)
          (Default|FlipArm (Variables|Default|GetMyPlayer))))
      (:then_1
        (Utilities|IsValid (Variables|UI|GetJigsawUI)
          (:Is%20Valid
            (CallFunction|JigsawDeactivate)
            (Default|JigsawL (Variables|Default|GetLastHoldedKeyItem)))))
      (:then_2
        (Rendering|Components|TextRender|SetText (Variables|/Game/Blueprints/BP_FirstPersonCharacter.BP_FirstPersonCharacter_C|GetBPM (Variables|Default|GetMyPlayer)) (Utilities|Text|ToText(Integer) (+ (- (Variables|Stress|GetStressMax) (Variables|Stress|GetCurrentStress)) 80)))))))

(fn GainStress
  (params (AmountGained :type Integer))
  (Variables|Stress|SetCurrentStress (Math|Integer|Clamp(Integer) (+ (Variables|Stress|GetCurrentStress) AmountGained) 0 (Variables|Stress|GetStressMax)))
  (Default|UpdateStress (Variables|UI|GetSanityUI) (- 1.0 (Utilities|GetSanityPercent)))
  (Rendering|Components|TextRender|SetText (Variables|/Game/Blueprints/BP_FirstPersonCharacter.BP_FirstPersonCharacter_C|GetBPM (Variables|Default|GetMyPlayer)) (Utilities|Text|ToText(Integer) (+ (- (Variables|Stress|GetStressMax) (Variables|Stress|GetCurrentStress)) 80))))

(fn UpdateStressMarge
  (|SetValues)
  (Default|UpdateRecoveryRange (Variables|UI|GetRecoverUI) (Variables|RecoverGame|GetRecoverRangeMin) (Variables|RecoverGame|GetRecoverRangeMax)))